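; Movement controller component for BP_Crocodile that drives its Control Rig for procedural crawling and terrain-following body animation.
; It configures four leg controllers with staggered phases for a crawl gait.
; On a timed interval it raycasts below spine controls for surface-offset targets, interpolating toward them each tick with hip-motion compensation.
; Each tick it also yaws the breast control from the leg-pair phase difference; body sway, hip rotation and forward-force functions are currently unused.
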(event Custom|InitializeLegControllers
  (params (LeftLeg :type BP%20Leg%20Controller%20Object%20Reference) (RightLeg :type BP%20Leg%20Controller%20Object%20Reference) (LeftLimb :type BP%20Leg%20Controller%20Object%20Reference) (RightLimb :type BP%20Leg%20Controller%20Object%20Reference))
  (Variables|Default|SetLeftLeg LeftLeg)
  (Variables|Default|SetRightLeg RightLeg)
  (Variables|Default|SetLeftLimb LeftLimb)
  (Variables|Default|SetRightLimb RightLimb)
  (EventDispatchers|BindEventtoOnPerformingStep (Variables|Default|GetLeftLeg) (EventDispatchers|CreateEvent :!event Custom|PerformingStep))
  (EventDispatchers|BindEventtoOnPerformingStep (Variables|Default|GetRightLeg) (EventDispatchers|CreateEvent :!event Custom|PerformingStep))
  (EventDispatchers|BindEventtoOnPerformingStep (Variables|Default|GetLeftLimb) (EventDispatchers|CreateEvent :!event Custom|PerformingStep))
  (EventDispatchers|BindEventtoOnPerformingStep (Variables|Default|GetRightLimb) (EventDispatchers|CreateEvent :!event Custom|PerformingStep))
  (CallFunction|InitializeAdditionalControllers)
  (Variables|/Game/Blueprints/BP_LegController.BP_LegController_C|SetDeleteThisHeight (Variables|Default|GetLeftLimb) "0.000000,0.000000,5.000000")
  (Variables|/Game/Blueprints/BP_LegController.BP_LegController_C|SetDeleteThisHeight (Variables|Default|GetRightLimb) "0.000000,0.000000,5.000000"))

(event Custom|StartCrawlGait
  (params (speed :type Float%20%28double-precision%29))
  ;[1 1 1] Initializing Movement with Crawl pattern and current speed
  (Utilities|FlowControl|Sequence
    (:then_0
      (Variables|/Game/Blueprints/BP_LegController.BP_LegController_C|SetOneStepCycleInSeconds (Variables|Default|GetLeftLeg) (Variables|Parameters|GetOneStepCycleInSecs))
      (Variables|/Game/Blueprints/BP_LegController.BP_LegController_C|SetOneStepCycleInSeconds (Variables|Default|GetLeftLimb) (Variables|Parameters|GetOneStepCycleInSecs))
      (Variables|/Game/Blueprints/BP_LegController.BP_LegController_C|SetOneStepCycleInSeconds (Variables|Default|GetRightLeg) (Variables|Parameters|GetOneStepCycleInSecs))
      (Variables|/Game/Blueprints/BP_LegController.BP_LegController_C|SetOneStepCycleInSeconds (Variables|Default|GetRightLimb) (Variables|Parameters|GetOneStepCycleInSecs)))
    (:then_1
      (Default|InitializeLegwithValuesandState (Variables|Default|GetLeftLimb) 0.15 "NewEnumerator2" 0.35 0.0)
      (Default|InitializeLegwithValuesandState (Variables|Default|GetRightLeg) 0.15 "NewEnumerator1" 0.35 0.0)
      (Default|InitializeLegwithValuesandState (Variables|Default|GetLeftLeg) 0.5 "NewEnumerator0" 0.35 0.0)
      (Default|InitializeLegwithValuesandState (Variables|Default|GetRightLimb) 0.65 "NewEnumerator0" 0.35 0.0))))

(event Custom|PerformingStep
  (params (LegType :type E_LegType%20Enum :default "NewEnumerator0") (PercentageReplanted :type Float%20%28double-precision%29)))

(event Custom|InitializeAdditionalControllers
  (Variables|Default|SetTopSpineJoint (Class|ControlRigComponent|GetControlRotator (Variables|Default|GetControlRig) "NeckRotationCtrl" "LocalSpace")))

(event EventBeginPlay
  (Utilities|FlowControl|DelayUntilNextTick)
  (bind _asbp_crocodile (Utilities|Casting|CastToBP_Crocodile (Components|GetOwner)))
  (Variables|Default|SetControlRig (Variables|/Game/Blueprints/BP_Crocodile.BP_Crocodile_C|GetControlRig _asbp_crocodile)))

(event EventTick
  (params (DeltaSeconds :type Float%20%28single-precision%29))
  (Utilities|FlowControl|Sequence
    (:then_0
      ;[1 1 1] Delay
      (Variables|Service|SetCurrentTimeDelayAlign (+ (Variables|Service|GetCurrentTimeDelayAlign) (Utilities|Time|GetWorldDeltaSeconds)))
      (if (> (Variables|Service|GetCurrentTimeDelayAlign) (Variables|Default|GetTimeDelayAlign))
        (Variables|Service|SetCurrentTimeDelayAlign 0.0)
        (CallFunction|AlligntoSurface)))
    (:then_1
      (CallFunction|InterpolateSplineTransforms))
    (:then_2
      (CallFunction|PerformNeckRotation))))

(fn PerformNeckRotation
  (bind _controlrig (Variables|Default|GetControlRig))
  (bind _leftleg (Variables|Default|GetLeftLeg))
  (bind _rightleg (Variables|Default|GetRightLeg))
  (Utilities|IsValid _controlrig
    (:Is%20Valid
      (Class|ControlRigComponent|SetControlTransform _controlrig "TA_Crocodile_Breast" (Math|Transform|MakeTransform "0, 0, 0" (Math|Rotator|MakeRotator 0.0 0.0 (* (- (- (/ (Variables|/Game/Blueprints/BP_LegController.BP_LegController_C|GetCurrentStepLengthSeconds _leftleg) (Variables|/Game/Blueprints/BP_LegController.BP_LegController_C|GetStepLengthSeconds _leftleg)) (/ (Variables|/Game/Blueprints/BP_LegController.BP_LegController_C|GetTimeSinceUnplanted _leftleg) (Variables|/Game/Blueprints/BP_LegController.BP_LegController_C|GetSwingStepTime _leftleg))) (- (/ (Variables|/Game/Blueprints/BP_LegController.BP_LegController_C|GetCurrentStepLengthSeconds _rightleg) (Variables|/Game/Blueprints/BP_LegController.BP_LegController_C|GetStepLengthSeconds _rightleg)) (/ (Variables|/Game/Blueprints/BP_LegController.BP_LegController_C|GetTimeSinceUnplanted _rightleg) (Variables|/Game/Blueprints/BP_LegController.BP_LegController_C|GetSwingStepTime _rightleg)))) (Variables|Parameters|GetNeckAngleRotationMax) -1.0)) "1.000000,1.000000,1.000000") "RigSpace"))))

(fn PerformBodyRotation
  (bind _output_get (Variables|Default|SetTotalTime (+ (Variables|Default|GetTotalTime) (Utilities|Time|GetWorldDeltaSeconds))))
  (LocalVariables|SetCurveValue (Math|Curves|GetFloatValue (Variables|Parameters|GetNeckRotationCurve) (* (/ (.Remainder (Math|Float|Division(WholeandRemainder) _output_get (Variables|Parameters|GetOneStepCycleInSecs))) (Variables|Parameters|GetOneStepCycleInSecs)) 2.0)))
  (Class|ControlRigComponent|SetControlRotator (Variables|Default|GetControlRig) "BodyRotationCtrl2" (Math|Rotator|MakeRotator 0.0 0.0 (* (LocalVariables|GetCurveValue) -15.0)) "LocalSpace")
  (Class|ControlRigComponent|SetControlRotator (Variables|Default|GetControlRig) "BodyHarmonics" (Math|Rotator|MakeRotator (+ (* (LocalVariables|GetCurveValue) -5.0) 9e+01) (* (LocalVariables|GetCurveValue) 1e+01) 0.0) "LocalSpace"))

(fn GetSurfaceLocation
  (params (RaycastControlName :type Name))
  (Utilities|FlowControl|Sequence
    (:then_0
      (LocalVariables|SetRayStart (Class|ControlRigComponent|GetControlPosition (Variables|Default|GetControlRig) RaycastControlName "WorldSpace")))
    (:then_1
      (LocalVariables|SetRayEnd (+ (LocalVariables|GetRayStart) (LocalVariables|GetRayLength))))
    (:then_2
      (bind (_location _normal) (Utilities|CastRay (LocalVariables|GetRayStart) (LocalVariables|GetRayEnd))
        (:True
          (return _location _normal))
        (:False
          (return "0, 0, 0" "0.000000,0.000000,1.000000"))))))

(fn AlligntoSurface
  (Utilities|Map|Clear (Variables|Service|GetNewSplineTransforms))
  (Class|ControlRigComponent|SetControlFloat (Variables|Default|GetControlRig) "S_AlphaInterpolation" 0.0)
  (for _array_element (LocalVariables|GetControlNames)
    (bind (_location _normal) (Utilities|CastRay (.location (Class|ControlRigComponent|GetControlTransform (Variables|Default|GetControlRig) (Utilities|String|StringToName (Utilities|String|BuildString(Name) "RC_" "" _array_element "")) "WorldSpace")) (- (.location (Class|ControlRigComponent|GetControlTransform (Variables|Default|GetControlRig) (Utilities|String|StringToName (Utilities|String|BuildString(Name) "RC_" "" _array_element "")) "WorldSpace")) "0.000000,0.000000,5000.000000"))
      (:True
        (Utilities|Map|Add (Variables|Service|GetNewSplineTransforms) (Utilities|String|StringToName (Utilities|String|BuildString(Name) "TA_" "" _array_element "")) (+ _location (* _normal (Variables|Parameters|GetPelvisHeight))))
        (Utilities|Map|Add (Variables|Service|GetPrevSplineTransforms) (Utilities|String|StringToName (Utilities|String|BuildString(Name) "TA_" "" _array_element "")) (.location (Class|ControlRigComponent|GetControlTransform (Variables|Default|GetControlRig) (Utilities|String|StringToName (Utilities|String|BuildString(Name) "TA_" "" _array_element "")) "WorldSpace")))
        (Variables|Service|SetPreviousHipPos (.location (Transformation|GetBoneTransform (Variables|Default|GetControlRig) "Crocodile_Hip" "WorldSpace")))))))

(fn AngleBetween2Vectors
  (params (Vec1 :type Vector) (Vec2 :type Vector))
  (return (Class|KismetMathLibrary|DegAcos (Math|Vector|DotProduct (Math|Vector|Normalize Vec1) (Math|Vector|Normalize Vec2)))))

(fn GetBoneRotation
  (params (BoneVector :type Vector) (SurfaceNormal :type Vector))
  (bind _returnvalue (Math|Vector|CrossProduct BoneVector SurfaceNormal))
  (bind _returnvalue_2 (Math|Vector|CrossProduct _returnvalue SurfaceNormal))
  (bind _returnvalue_3 (Math|Vector|Normalize _returnvalue_2))
  (Utilities|FlowControl|Sequence
    (:then_0
      (Class|KismetMathLibrary|VectorNormalize BoneVector 1e-05)
      (Class|KismetMathLibrary|VectorNormalize SurfaceNormal 1e-05))
    (:then_1
      (LocalVariables|SetNewBoneVector _returnvalue_3)
      (if (< (Math|Vector|DotProduct _returnvalue_3 BoneVector) 0.0)
        (LocalVariables|SetNewBoneVector (* (LocalVariables|GetNewBoneVector) -1.0)))
      (bind _rotator (CallFunction|Rotatorfrom2Vectors BoneVector (LocalVariables|GetNewBoneVector)))
      (return (Math|Rotator|MakeRotator (.roll _rotator) (.yaw _rotator) 0.0)))))

(fn Rotatorfrom2Vectors
  (params (Vec1 :type Vector) (Vec2 :type Vector))
  (if (Utilities|Operators|EqualEqual Vec1 Vec2 1e-05)
    (return (Class|KismetMathLibrary|QuatRotator (Class|KismetMathLibrary|QuatIdentity)))
    (else
      (bind _angle (CallFunction|AngleBetween2Vectors Vec1 Vec2))
      (return (Math|Vector|RotatorfromAxisandAngle (Math|Vector|Normalize (Math|Vector|CrossProduct Vec1 Vec2)) _angle)))))

(fn Move
  (bind _output_get (Variables|Default|SetMoveDirection (Math|Vector|Normalize (- (.location (Transformation|GetBoneTransform (Variables|Default|GetControlRig) "Crocodile_Neck_02SHJnt" "WorldSpace")) (.location (Transformation|GetBoneTransform (Variables|Default|GetControlRig) "Crocodile_Spine_TopSHJnt" "WorldSpace"))))))
  (bind _asbp_crocodile (Utilities|Casting|CastToBP_Crocodile (Components|GetOwner)))
  (Physics|AddForce (Variables|/Game/Blueprints/BP_Crocodile.BP_Crocodile_C|GetCapsule _asbp_crocodile) (* _output_get 2e+01) "None" true))

(fn InterpolateSplineTransforms
  (Utilities|FlowControl|Sequence
    (:then_0
      (for _array_element (LocalVariables|GetControlNames)
        (Class|ControlRigComponent|SetControlTransform (Variables|Default|GetControlRig) (Utilities|String|StringToName (Utilities|String|BuildString(Name) "TA_" "" _array_element "")) (Math|Transform|MakeTransform (+ (Math|Vector|Lerp(Vector) (.Value (Utilities|Map|Find (Variables|Service|GetPrevSplineTransforms) (Utilities|String|StringToName (Utilities|String|BuildString(Name) "TA_" "" _array_element "")))) (.Value (Utilities|Map|Find (Variables|Service|GetNewSplineTransforms) (Utilities|String|StringToName (Utilities|String|BuildString(Name) "TA_" "" _array_element "")))) (/ (Variables|Service|GetCurrentTimeDelayAlign) (Variables|Default|GetTimeDelayAlign))) (- (.location (Transformation|GetBoneTransform (Variables|Default|GetControlRig) "Crocodile_Hip" "WorldSpace")) (Variables|Service|GetPreviousHipPos))) "0, 0, 0" "1.000000,1.000000,1.000000") "WorldSpace")))
    (:then_1
      (Class|ControlRigComponent|SetControlFloat (Variables|Default|GetControlRig) "S_AlphaInterpolation" (/ (Variables|Service|GetCurrentTimeDelayAlign) (Variables|Default|GetTimeDelayAlign))))))

(fn PerformHipsRotation
  (bind _rightlimb (Variables|Default|GetRightLimb))
  (bind _leftlimb (Variables|Default|GetLeftLimb))
  (Class|ControlRigComponent|SetControlOffset (Variables|Default|GetControlRig) "TA_Crocodile_Breast" (Math|Transform|MakeTransform "0, 0, 0" (Math|Rotator|MakeRotator 0.0 0.0 (+ (* (/ (Variables|/Game/Blueprints/BP_LegController.BP_LegController_C|GetTimeSinceUnplanted _rightlimb) (Variables|/Game/Blueprints/BP_LegController.BP_LegController_C|GetSwingStepTime _rightlimb)) -2e+01) (* (/ (Variables|/Game/Blueprints/BP_LegController.BP_LegController_C|GetTimeSinceUnplanted _leftlimb) (Variables|/Game/Blueprints/BP_LegController.BP_LegController_C|GetSwingStepTime _leftlimb)) 2e+01))) "1.000000,1.000000,1.000000") "WorldSpace"))