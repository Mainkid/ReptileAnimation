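; Per-leg controller for BP_Crocodile that drives procedural stepping of one foot through the owner's Control Rig.
; A tick state machine traces from a rig control for a target, swings the foot there with a lerp plus height curve, then pins it while calling the owner's Move.
; Swing and stance durations split one step cycle, rescalable mid-step.
; Replanting is unconditional, and ground normals reach the rig for only one leg type.
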(event EventBeginPlay
  (Utilities|FlowControl|DelayUntilNextTick)
  (bind _asbp_crocodile (Utilities|Casting|CastToBP_Crocodile (Components|GetOwner)))
  (Variables|Default|SetOwner _asbp_crocodile)
  (Variables|Default|SetControlRig (Variables|/Game/Blueprints/BP_Crocodile.BP_Crocodile_C|GetControlRig _asbp_crocodile)))

(event EventTick
  (params (DeltaSeconds :type Float%20%28single-precision%29))
  (Utilities|FlowControl|DelayUntilNextTick)
  (switch Utilities|FlowControl|Switch|SwitchonE_LegState (Variables|Default|GetLegState)
    (:NewEnumerator0
      (CallFunction|PlacedFootUpdate)
      (Variables|Default|SetStepTimeCurrent (+ (Variables|Default|GetStepTimeCurrent) (Utilities|Time|GetWorldDeltaSeconds)) :!label _label))
    (:NewEnumerator1
      (CallFunction|PerformStep)
      (goto _label))
    (:NewEnumerator2
      (CallFunction|GetFootTargetLocation)
      (CallFunction|CheckforReplant)
      (Variables|Default|SetStepTimeCurrent 0.0))))

(fn GetFootTargetLocation
  (bind _controlrig (Variables|Default|GetControlRig))
  (bind _raycastname (Variables|Parameters|GetRayCastName))
  (bind _returnvalue (Class|ControlRigComponent|GetControlTransform _controlrig _raycastname "WorldSpace"))
  (Utilities|FlowControl|Sequence
    (:then_0
      (LocalVariables|SetRayStart (.location _returnvalue)))
    (:then_1
      (LocalVariables|SetRayEnd (+ (LocalVariables|GetRayStart) (* (Math|Vector|GetUpVector (.rotation _returnvalue)) 1.0 4.5e+02))))
    (:then_2
      (bind (_location _normal) (Utilities|CastRay (LocalVariables|GetRayStart) (LocalVariables|GetRayEnd))
        (:True
          (bind _output_get (Variables|Default|SetTargetPosition _location))
          (CallFunction|PlaceFootNormal _normal)
          (return _output_get))
        (:False
          (return "0, 0, 0"))))))

(fn CheckforReplant
  ;[1 1 1] Добавить проверки!
  (Utilities|FlowControl|Sequence
    (:then_2
      (Variables|Default|SetLegState "NewEnumerator1")
      (Variables|Default|SetPlantStartPosition (Class|ControlRigComponent|GetControlPosition (Variables|Default|GetControlRig) (Variables|Parameters|GetControlName) "WorldSpace")))))

(fn PerformStep
  (Utilities|FlowControl|Sequence
    (:then_0
      (LocalVariables|SetPercentageReplanted (/ (Variables|Default|GetTimeSinceUnplanted) (Variables|Parameters|GetSwingStepTime))))
    (:then_1
      (Variables|Default|SetFootPositionNoHeight (Math|Vector|Lerp(Vector) (Variables|Default|GetPlantStartPosition) (Variables|Default|GetTargetPosition) (LocalVariables|GetPercentageReplanted))))
    (:then_2
      (Variables|Default|SetFootPosition (+ (+ (Variables|Default|GetFootPositionNoHeight) (Math|Vector|MakeVector 0.0 0.0 (* (Math|Curves|GetFloatValue (Variables|Parameters|GetLegHeightCurve) (LocalVariables|GetPercentageReplanted)) (Variables|Parameters|GetStepHeight)))) (Variables|Default|GetDeleteThisHeight))))
    (:then_3
      (if (>= (Variables|Default|GetTimeSinceUnplanted) (Variables|Parameters|GetSwingStepTime))
        (Variables|Default|SetLegState "NewEnumerator0")
        (else
          (Class|ControlRigComponent|SetControlTransform (Variables|Default|GetControlRig) (Variables|Parameters|GetControlName) (Math|Transform|MakeTransform (Variables|Default|GetFootPosition) "0, 0, 0" "1.000000,1.000000,1.000000") "WorldSpace")
          (Variables|Default|SetTimeSinceUnplanted (+ (Utilities|Time|GetWorldDeltaSeconds) (Variables|Default|GetTimeSinceUnplanted))))))
    (:then_4
      (Default|CallOnPerformingStep (Variables|Default|GetCurrentLegType) (LocalVariables|GetPercentageReplanted)))))

(fn RefreshValues
  (Variables|Default|SetLegState "NewEnumerator2")
  (Variables|Default|SetTimeSinceUnplanted 0.0)
  (Variables|Default|SetTargetPosition "0, 0, 0")
  (Variables|Default|SetFootPositionNoHeight "0, 0, 0")
  (Variables|Default|SetCurrentStepLengthSeconds 0.0))

(fn PlacedFootUpdate
  (Variables|Default|SetCurrentStepLengthSeconds (+ (Variables|Default|GetCurrentStepLengthSeconds) (Utilities|Time|GetWorldDeltaSeconds)))
  (if (<= (Variables|Default|GetCurrentStepLengthSeconds) (Variables|Parameters|GetStepLengthSeconds))
    (Class|ControlRigComponent|SetControlTransform (Variables|Default|GetControlRig) (Variables|Parameters|GetControlName) (Math|Transform|MakeTransform (Variables|Default|GetFootPosition) "0, 0, 0" "1.000000,1.000000,1.000000") "WorldSpace")
    (Default|Move (Variables|Default|GetOwner))
    (else
      (CallFunction|RefreshValues))))

(fn InitializeLegwithValuesandState
  (params (percentageOfPlantedVar :type Float%20%28double-precision%29) (legStateVar :type E_LegState%20Enum :default "NewEnumerator0") (swingPhaseLengthPercentage :type Float%20%28double-precision%29) (TimeSinceUnplantedVar :type Float%20%28double-precision%29))
  (Variables|Default|SetLegState legStateVar)
  (bind _output_get (Variables|Parameters|SetStepLengthSeconds (* (Variables|Parameters|GetOneStepCycleInSeconds) (- 1.0 swingPhaseLengthPercentage))))
  (Variables|Default|SetCurrentStepLengthSeconds (* percentageOfPlantedVar _output_get))
  (Variables|Parameters|SetSwingStepTime (* (Variables|Parameters|GetOneStepCycleInSeconds) swingPhaseLengthPercentage))
  (Variables|Default|SetTimeSinceUnplanted TimeSinceUnplantedVar)
  (Variables|Default|SetSwingPhaseLengthPercents swingPhaseLengthPercentage))

(fn UpdateSwingsandStepTime
  (params (NewStepCycleInSecs :type Float%20%28double-precision%29))
  (bind _swingphaselengthpercents (Variables|Default|GetSwingPhaseLengthPercents))
  (Variables|Default|SetCurrentStepLengthSeconds (* (Variables|Default|GetCurrentStepLengthSeconds) (/ NewStepCycleInSecs (Variables|Parameters|GetOneStepCycleInSeconds))))
  (Variables|Default|SetTimeSinceUnplanted (* (Variables|Default|GetTimeSinceUnplanted) (/ NewStepCycleInSecs (Variables|Parameters|GetOneStepCycleInSeconds))))
  (Variables|Parameters|SetOneStepCycleInSeconds NewStepCycleInSecs)
  (Variables|Parameters|SetSwingStepTime (* (Variables|Parameters|GetOneStepCycleInSeconds) _swingphaselengthpercents))
  (Variables|Parameters|SetStepLengthSeconds (* (Variables|Parameters|GetOneStepCycleInSeconds) (- 1.0 _swingphaselengthpercents))))

(fn PlaceFootNormal
  (params (Normal :type Vector))
  (bind _asnew_control_rig_blueprint (Utilities|Casting|CastToNewControlRigBlueprint (Class|ControlRigComponent|GetControlRig (Variables|/Game/Blueprints/BP_Crocodile.BP_Crocodile_C|GetControlRig (Variables|Default|GetOwner)))))
  (if (Utilities|Enum|Equal(Enum) (Variables|Default|GetCurrentLegType) "NewEnumerator0")
    (bind _output_get (Variables|/Game/NewControlRigBlueprint.NewControlRigBlueprint_C|SetLeftFrontLegNormal _asnew_control_rig_blueprint Normal))
    (Development|PrintString (Utilities|String|ToString(Vector) _output_get))))